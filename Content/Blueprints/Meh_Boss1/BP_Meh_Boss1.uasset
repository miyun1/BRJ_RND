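; Side-view boss character with a viewport health bar, damage knockback, a death animation, and a Hit event that shakes the camera.
; Tick flips control rotation and Direction from horizontal velocity, updates the bar from Health, and sets IsDead when it empties.
; AnyDamage subtracts health and launches the boss using Direction, disabling movement and jumping to Dying only if IsDead was already set.
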(event Custom|Test%20Tick
  (params (DeltaSeconds :type Float%20%28single-precision%29))
  (Progress|SetPercent (Variables|/Game/Blueprints/Meh_Boss1/WB_Meh_Boss1_HealthBar.WB_Meh_Boss1_HealthBar_C|GetHealthBar (Variables|Default|GetHealthUI)) (/ (Variables|Default|GetHealth) 1e+02))
  (if (<= (Variables|/Script/UMG.ProgressBar|GetPercent (Variables|/Game/Blueprints/Meh_Boss1/WB_Meh_Boss1_HealthBar.WB_Meh_Boss1_HealthBar_C|GetHealthBar (Variables|Default|GetHealthUI))) 0.0)
    (Variables|Default|SetisDead true)))

(event Game|Damage|EventAnyDamage
  (params (Damage :type Float%20%28single-precision%29) (DamageType :type Damage%20Type%20Object%20Reference) (InstigatedBy :type Controller%20Object%20Reference) (DamageCauser :type Actor%20Object%20Reference))
  (bind _launchdistance (Variables|Default|GetlaunchDistance))
  (bind _output_get (Variables|Default|SetHealth (- (Variables|Default|GetHealth) Damage)))
  (Development|PrintString (Utilities|String|ToString(Float) _output_get))
  (bind _result (Math|Float|NegateFloat (* _launchdistance (Variables|Default|Getdirection)))
    (:%20%20
      (Components|Movement|StopMovementImmediately (Variables|Character|GetCharacterMovement))
      (Character|LaunchCharacter (Math|Vector|MakeVector _result 0.0 _launchdistance) false false)
      (if (Variables|Default|GetisDead)
        (Pawn|Components|CharacterMovement|DisableMovement (Variables|Character|GetCharacterMovement))
        (Class|PaperZDAnimInstance|JumptoNode (Variables|/Script/PaperZD.PaperZDAnimationComponent|GetAnimInstance (Variables|Default|GetAnimationComponent)) "Dying" "None")))))

(event Collision|EventActorBeginOverlap
  (params (OtherActor :type Actor%20Object%20Reference)))

(event EventHit
  ;[1 1 1] Attack
  (Utilities|FlowControl|Sequence
    (:then_0
      (Development|PrintString "HIT!"))
    (:then_1
      (Camera|PlayWorldCameraShake "/Game/Blueprints/Meh_Boss1/BP_Meh_CameraShake.BP_Meh_CameraShake_C" (Transformation|GetActorLocation) 0.0 3.5e+03))))

(event EventBeginPlay
  ;[1 1 1] Boss HealthBar
  (bind _returnvalue (UserInterface|CreateWidget "/Game/Blueprints/Meh_Boss1/WB_Meh_Boss1_HealthBar.WB_Meh_Boss1_HealthBar_C"))
  (UserInterface|Viewport|AddtoViewport _returnvalue 0)
  (Variables|Default|SetHealthUI _returnvalue))

(event EventTick
  (params (DeltaSeconds :type Float%20%28single-precision%29))
  (bind _returnvalue (Pawn|GetController))
  (bind _returnvalue_2 (Pawn|GetController))
  (CallFunction|TestTick DeltaSeconds)
  (|CallParentFunction DeltaSeconds)
  (Math|Float|CompareFloat (.X (Math|Vector|BreakVector (Variables|/Script/Engine.MovementComponent|GetVelocity (Pawn|GetMovementComponent)))) 0.0
    (:>
      ;[0 0.4745 1] Look Right
      (Utilities|IsValid _returnvalue_2
        (:Is%20Valid
          (Pawn|SetControlRotation _returnvalue_2 (Math|Rotator|MakeRotator 0.0 0.0 0.0))
          (Variables|Default|Setdirection 1.0))))
    (:<
      ;[0 0.4745 1] Look Left
      (Utilities|IsValid _returnvalue
        (:Is%20Valid
          (Pawn|SetControlRotation _returnvalue (Math|Rotator|MakeRotator 0.0 0.0 1.8e+02))
          (Variables|Default|Setdirection -1.0))))))

(fn ConstructionScript)