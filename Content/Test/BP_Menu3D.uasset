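; BP_Menu3D is a test 3D menu actor that hosts a UI_TestMenu3D widget and links to other menus.
; On BeginPlay it binds to the widget's transition event and disables its own collision.
; A menu index from the widget selects a LinkedMenus entry, which gains collision as this menu loses it.
; The player's view target then blends to the new menu with an eased camera move.
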(event Custom|TransitionTo
  (params (newMenu :type BP%20Menu%203D%20Object%20Reference))
  (Collision|SetActorEnableCollision false)
  (Collision|SetActorEnableCollision newMenu true)
  (Game|Player|SetViewTargetwithBlend (Game|GetPlayerController 0) newMenu 2.0 "VTBlend_EaseInOut" 2.0 false))

(event Custom|TransitionToLinkedMenu_Event
  (params (menuIndex :type Integer))
  (if (Utilities|Array|IsValidIndex (Variables|Default|GetLinkedMenus) menuIndex)
    (CallFunction|Transitionto (Utilities|Array|Get(acopy) (Variables|Default|GetLinkedMenus) menuIndex))))

(event EventBeginPlay
  (bind _asui_test_menu_3d (Utilities|Casting|CastToUI_TestMenu3D (UserInterface|GetUserWidgetObject (Variables|Default|GetWidget))))
  (EventDispatchers|AssignTransitiontoLinkedMenu _asui_test_menu_3d (delegate Custom|TransitionToLinkedMenu_Event))
  (Collision|SetActorEnableCollision false))

(fn ConstructionScript)